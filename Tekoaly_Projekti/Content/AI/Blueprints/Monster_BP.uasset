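; Monster AI pawn that wanders to random reachable points and chases the player character (ElvisRef) on sight.
; Pawn sensing flags danger and, unless the player is invisible, starts a distance-gated AIMoveTo that sets CanAttack and re-triggers itself on success.
; Tick drives patrol, a loose X/Y proximity check and smoothed yaw toward the player when close or attacking.
; Proximity gates the throttled chase sound; a retriggerable delay or PlayerKilled restores patrol.
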(event OnSeePawn(PawnSensing)
  (params (Pawn :type Pawn%20Object%20Reference))
  (bind _asbp_third_person_character (Utilities|Casting|CastToBP_ThirdPersonCharacter Pawn))
  (Variables|Default|SetElvis%20Ref _asbp_third_person_character)
  (Variables|/Game/ThirdPerson/Blueprints/BP_ThirdPersonCharacter.BP_ThirdPersonCharacter_C|SetMonsterDanger (Variables|Default|GetElvis%20Ref) true)
  (Utilities|FlowControl|Sequence
    (:then_0
      (Variables|Default|SetPatrol false)
      (if (Variables|/Game/ThirdPerson/Blueprints/BP_ThirdPersonCharacter.BP_ThirdPersonCharacter_C|GetInvisibleMode (Variables|Default|GetElvis%20Ref))
        (Variables|Default|SetPatrol true)
        (else
          (Utilities|FlowControl|Sequence
            (:then_0
              (if (< (Math|Vector|Distance(Vector) (Transformation|GetWorldLocation (Variables|Character|GetMesh)) (Transformation|GetActorLocation (Variables|Default|GetElvis%20Ref))) 2e+03)
                (AI|AIMoveTo self "0, 0, 0" (Variables|Default|GetElvis%20Ref) 1e+02 false
                  (:OnSuccess
                    (Variables|Default|SetcanAttack true)
                    (Utilities|FlowControl|Delay 0.3)
                    (CallFunction|GotoPlayer)
                    (Utilities|FlowControl|Delay 3.0)
                    (Variables|Default|SetcanAttack false))
                  (:OnFail
                    (Variables|Default|SetcanAttack false)))))
            (:then_1
              (if (Variables|Default|GetCloseToPlayer)
                (Utilities|FlowControl|DoOnce false :!label _label
                  (:Completed
                    (Audio|PlaySound2D "/Game/Sounds/Zombie/Chase_Cue.Chase_Cue" 0.1 1.0 0.0 0 0)
                    (Utilities|FlowControl|Delay 5.0)
                    (goto _label Reset)))
                (else
                  (Variables|Default|SetPatrol true))))))))
    (:then_1
      (Utilities|FlowControl|RetriggerableDelay 3.0)
      (Variables|Default|SetPatrol true))))

(event Custom|Player%20Killed
  (Variables|Default|SetcanAttack false)
  (Variables|Default|SetPatrol true))

(event Custom|GoToPlayer
  (if (< (Math|Vector|Distance(Vector) (Transformation|GetWorldLocation (Variables|Character|GetMesh)) (Transformation|GetActorLocation (Variables|Default|GetElvis%20Ref))) 2e+03)
    (AI|AIMoveTo self "0, 0, 0" (Variables|Default|GetElvis%20Ref) 1e+02 false
      (:OnSuccess
        (Variables|Default|SetcanAttack true)
        (Utilities|FlowControl|Delay 0.3)
        (CallFunction|GotoPlayer)
        (Utilities|FlowControl|Delay 3.0)
        (Variables|Default|SetcanAttack false))
      (:OnFail
        (Variables|Default|SetcanAttack false)))))

(event EventBeginPlay
  (bind _asbp_third_person_character (Utilities|Casting|CastToBP_ThirdPersonCharacter (Game|Player|GetPlayerPawn 0)))
  (Variables|Default|SetElvis%20Ref _asbp_third_person_character))

(event Collision|EventActorBeginOverlap
  (params (OtherActor :type Actor%20Object%20Reference)))

(event EventTick
  (params (DeltaSeconds :type Float%20%28single-precision%29))
  (bind _returnvalue (Transformation|GetActorLocation))
  (bind _elvis_ref (Variables|Default|GetElvis%20Ref))
  (bind _returnvalue_2 (Transformation|GetActorLocation _elvis_ref))
  (bind _returnvalue_3 (- (.x _returnvalue) (.x _returnvalue_2)))
  (bind _returnvalue_4 (- (.y _returnvalue) (.y _returnvalue_2)))
  (Utilities|FlowControl|Sequence
    (:then_0
      (if (Variables|Default|GetPatrol)
        (Utilities|FlowControl|Sequence
          (:then_1
            (Utilities|FlowControl|Delay (Math|Random|RandomFloatinRange 2.0 5.0))
            (AI|AIMoveTo self (.RandomLocation (AI|Navigation|GetRandomReachablePointinRadius (Transformation|GetActorLocation) 2e+03 0 0)) 0 5.0 false)))))
    (:then_1
      (if (or (>= _returnvalue_4 -1e+03) (>= _returnvalue_3 -1e+03))
        (if (or (<= _returnvalue_4 1e+03) (<= _returnvalue_3 1e+03))
          (Variables|Default|SetCloseToPlayer true)
          (else
            (Variables|Default|SetCloseToPlayer false :!label _label)))
        (else
          (goto _label))))
    (:then_3
      (if (Variables|Default|GetCloseToPlayer)
        (Transformation|SetActorRotation (Math|Rotator|MakeRotator 0.0 0.0 (.yaw (Math|Interpolation|RInterpTo (Transformation|GetActorRotation) (Math|Rotator|FindLookatRotation (Transformation|GetActorLocation) (Transformation|GetActorLocation (Variables|Default|GetElvis%20Ref))) (Utilities|Time|GetWorldDeltaSeconds) 1e+01))) :!label _label_2)
        (elif (Variables|Default|GetCanAttack)
          (goto _label_2))))))

(fn ConstructionScript)