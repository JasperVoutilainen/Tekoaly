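; Zombie enemy locked to a fixed X plane for side-on movement, which patrols random nearby points and chases seen pawns.
; Pawn sensing drives AI MoveTo, setting CanAttack on arrival and playing a throttled chase sound when near the player.
; Tick handles patrol, left/right facing, Y-axis proximity and death.
; Bullet damage lowers health; death disables movement and collision, spawns one actor via nested random MultiGates, then destroys the zombie.
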(event OnSeePawn(PawnSensing)
  (params (Pawn :type Pawn%20Object%20Reference))
  (Utilities|FlowControl|Sequence
    (:then_0
      (bind _asrifle_player_bp (Utilities|Casting|CastTo Pawn)
        (:then
          _)
        (:CastFailed
          (Variables|Default|SetPatrol false)))
      (if (< (Math|Vector|Distance(Vector) (Transformation|GetWorldLocation (Variables|Character|GetMesh)) (Transformation|GetActorLocation _asrifle_player_bp)) 1e+04)
        (AI|AIMoveTo self "0, 0, 0" _asrifle_player_bp 1.5e+02 false
          (:OnSuccess
            (Variables|Default|SetcanAttack true))
          (:OnFail
            (Variables|Default|SetcanAttack false)))
        (else
          (Variables|Default|SetPatrol true))))
    (:then_1
      (if (Variables|Default|GetCloseToPlayer)
        (if (not (Variables|Default|GetIsDead))
          (Utilities|FlowControl|DoOnce false :!label _label
            (:Completed
              (Audio|PlaySound2D "/Game/Sounds/Zombie/Chase_Cue.Chase_Cue" 0.1 1.0 0.0 0 0)
              (Utilities|FlowControl|Delay 5.0)
              (goto _label Reset))))))))

(event Custom|Player%20Killed
  (Variables|Default|SetcanAttack false))

(event Custom|BulletHits
  (params (Bullet%20Ref :type %20Object%20Reference))
  (Game|Damage|ApplyDamage self (Variables|Default|GetDamageFromBullet Bullet%20Ref) 0 0))

(event EventBeginPlay
  (Variables|Default|SetInitial%20X (.X (Math|Vector|BreakVector (Transformation|GetWorldLocation (Variables|Character|GetMesh)))))
  (Variables|Default|SetHealth (Variables|Default|GetHealth (Variables|Default|GetHealthComponent)))
  (bind _asrifle_player_bp (Utilities|Casting|CastTo (Game|GetPlayerCharacter 0)))
  (Variables|Default|SetRiflePlayer%20Ref 0 _asrifle_player_bp))

(event Game|Damage|EventAnyDamage
  (params (Damage :type Float%20%28single-precision%29) (DamageType :type Damage%20Type%20Object%20Reference) (InstigatedBy :type Controller%20Object%20Reference) (DamageCauser :type Actor%20Object%20Reference))
  (Variables|Default|SetHealth (- (Variables|Default|GetHealth) Damage)))

(event EventTick
  (params (DeltaSeconds :type Float%20%28single-precision%29))
  (bind _returnvalue (Transformation|GetActorLocation))
  (bind _rifleplayer_ref (Variables|Default|GetRiflePlayer%20Ref))
  (bind _mesh (Variables|Character|GetMesh))
  (bind _returnvalue_2 (Transformation|GetWorldLocation _mesh))
  (bind _returnvalue_3 (Transformation|GetActorLocation _rifleplayer_ref))
  (bind (_x _y _z) (Math|Vector|BreakVector _returnvalue_2))
  (bind _returnvalue_4 (- (.y _returnvalue) (.y _returnvalue_3)))
  (Utilities|FlowControl|Sequence
    (:then_0
      (if (Variables|Default|GetPatrol)
        (Utilities|FlowControl|Delay (Math|Random|RandomFloatinRange 2.0 5.0))
        (AI|AIMoveTo self (.RandomLocation (AI|Navigation|GetRandomReachablePointinRadius (Transformation|GetActorLocation) 5e+02 0 0)) 0 5.0 false)))
    (:then_1
      (if (Variables|Default|GetIsDead)
        (Utilities|FlowControl|DoOnce false
          (:Completed
            _)))
      (Transformation|SetRelativeRotation (Variables|Collision|GetCapsuleComponent) (Math|Rotator|MakeRotator 0.0 0.0 (select (<= (.y (Transformation|GetActorLocation (.RiflePlayer%20Ref (Variables|Default|GetRiflePlayer%20Ref)))) (.y (Transformation|GetActorLocation))) -9e+01 9e+01)) false false))
    (:then_2
      (Transformation|SetWorldLocation _mesh (Math|Vector|MakeVector (Variables|Default|GetInitial%20X) _y _z) false false))
    (:then_3
      (if (<= (Variables|Default|GetHealth) 0.0)
        (Utilities|FlowControl|DoOnce false
          (:Completed
            (Variables|Default|SetisSeeingPlayer false)
            (Variables|Default|SetcanAttack false)
            (Variables|Default|SetPatrol false)
            (Variables|Default|SetIsDead true)
            (if (Variables|Default|GetCloseToPlayer)
              (Audio|PlaySound2D 0 0.1 1.0 0.0 0 0)
              (else
                (Audio|PlaySound2D 0 0.0 1.0 0.0 0 0)))
            (Collision|SetCollisionEnabled (Variables|Collision|GetCapsuleComponent) "NoCollision")
            (Pawn|Components|CharacterMovement|DisableMovement (Variables|Character|GetCharacterMovement))
            (Utilities|FlowControl|MultiGate true false -1
              (:Out%200
                (Game|SpawnActorfromClass 0 (Math|Transform|MakeTransform (Transformation|GetActorLocation) "0, 0, 0" "0.100000,0.100000,0.100000") "Undefined" 0 0 :!label _label))
              (:Out%201
                (Utilities|FlowControl|MultiGate true false -1
                  (:Out%200
                    (goto _label))
                  (:Out%201
                    (Utilities|FlowControl|MultiGate true false -1
                      (:Out%200
                        (goto _label))
                      (:Out%201
                        (Game|SpawnActorfromClass 0 (Math|Transform|MakeTransform (Transformation|GetActorLocation) "0, 0, 0" "0.700000,0.700000,0.700000") "Undefined" 0 0)))))))
            (Utilities|FlowControl|Delay 5.0)
            (Actor|DestroyActor)))))
    (:then_4
      (if (>= _returnvalue_4 -1e+03)
        (if (<= _returnvalue_4 1e+03)
          (Variables|Default|SetCloseToPlayer true)
          (else
            (Variables|Default|SetCloseToPlayer false :!label _label_2)))
        (else
          (goto _label_2))))))

(fn ConstructionScript)